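; BP_Camera is a standalone camera rig that smoothly follows the player each tick, with its spring arm matching control rotation.
; A downward trace from the player's mesh sets the rig's height above the floor.
; Without floor, it holds the last floor height, switching to player height during wallruns (detected by gameplay tag) or hard falls.
; A DoOnce flags hard falls past a distance threshold and resets on landing.
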(event `self.ReceiveTick`
  (params (DeltaSeconds :type "Float (single-precision)"))
  (`self.AdjustSpringArm`))

(event `AdjustSpringArm`
  (bind (_lastimpactpoint_x _lastimpactpoint_y _lastimpactpoint_z) (`KismetMathLibrary.BreakVector` (`self.LastImpactPoint`)))
  (bind (_lastimpactpoint_x_2 _lastimpactpoint_y_2 _lastimpactpoint_z_2) (`KismetMathLibrary.BreakVector` (`self.LastImpactPoint`)))
  (bind (_returnvalue_x _returnvalue_y _returnvalue_z) (`KismetMathLibrary.BreakVector` (`self.K2_GetActorLocation` (`self.Player`))))
  (bind _returnvalue (`GameplayTagAssetInterface.HasMatchingGameplayTag` (`CLMCharacter.AbilitySystemComponent` (`self.Player`)) (struct :`TagName` "Wallrun.CharacterIsAttached")))
  (bind _returnvalue_2 (`SceneComponent.K2_GetComponentLocation` (`Character.Mesh` (`self.Player`))))
  (`self.Player`
    (:`then`
      (`|ExecutionSequence`
        (:`then_0`
          (`SceneComponent.K2_SetWorldRotation` (`self.SpringArm`) (`Pawn.GetControlRotation` (`self.Player`)) false false))
        (:`then_1`
          (bind _outhit (`KismetSystemLibrary.LineTraceSingle` _returnvalue_2 (- _returnvalue_2 (`KismetMathLibrary.MakeVector` 0.0 0.0 (`self.FloorCheckDist`))) "TraceTypeQuery1" false (`|MakeArray` (`self.Player`) :!type "Actor Object Reference")))
          (if (`GameplayStatics.BreakHitResult` _outhit)
            (set `self.LastImpactPoint` (`.ImpactPoint` (`GameplayStatics.BreakHitResult` _outhit)))
            (`self.K2_SetActorLocation` (`KismetMathLibrary.VInterpTo` (`self.K2_GetActorLocation`) (`KismetMathLibrary.MakeVector` _lastimpactpoint_x_2 _lastimpactpoint_y_2 (+ _lastimpactpoint_z_2 120.0)) (`GameplayStatics.GetWorldDeltaSeconds`) 15.0))
            (set `self.HardFalling` false)
            (`self.Reset`)
            (else
              (`|ExecutionSequence`
                (:`then_0`
                  (if (> (`KismetMathLibrary.Vector_Distance` (`self.K2_GetActorLocation` (`self.Player`)) (`self.K2_GetActorLocation`)) 180.0)
                    (`/Engine/EditorBlueprintResources/StandardMacros.DoOnce` false :!label _label
                      (:`Completed`
                        (set `self.HardFalling` true)))))
                (:`then_1`
                  (`self.K2_SetActorLocation` (`KismetMathLibrary.VInterpTo` (`self.K2_GetActorLocation`) (`KismetMathLibrary.MakeVector` _returnvalue_x _returnvalue_y (`KismetMathLibrary.SelectFloat` _returnvalue_z (+ _lastimpactpoint_z 120.0) (or _returnvalue (`self.HardFalling`)))) (`GameplayStatics.GetWorldDeltaSeconds`) 15.0))
                  (if _returnvalue
                    (set `self.LastImpactPoint` (`KismetMathLibrary.MakeVector` 0.0 0.0 _returnvalue_z))))))))))
    (:`else`)))

(event `Reset`
  (goto _label :!via `Reset`))

(fn `UserConstructionScript`)
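; Gameplay ability that makes the player character slide by playing a short slide montage.
; On commit it ignores GameTraceChannel1 on the capsule, hides the weapon_r bone and calls EnableSliding on BP_PlayerCharacter.
; The Event.Montage.Slide gameplay event or any montage exit ends the ability.
; OnEndAbility restores bone and collision, disables sliding and removes the loose State.Sliding tag, which is not added here.
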(event `self.K2_ActivateAbility`
  (bind _owner (`self.Owner`))
  (bind _returnvalue (`self.K2_CommitAbility`))
  (if _returnvalue
    (bind _asbp_player_character (cast `/Game/PlayerCharacter/Character/BP_PlayerCharacter` (`self.GetAvatarActorFromActorInfo`)))
    (set `self.Owner` _asbp_player_character)
    (`PrimitiveComponent.SetCollisionResponseToChannel` (`Character.CapsuleComponent` (`self.Owner`)) "ECC_GameTraceChannel1" "ECR_Ignore")
    (`SkinnedMeshComponent.HideBoneByName` (`Character.Mesh` (`self.Owner`)) "weapon_r" "PBO_None")
    (`/Game/PlayerCharacter/Character/BP_PlayerCharacter.EnableSliding` (`self.Owner`))
    (`AbilityTask_PlayMontageAndWait.CreatePlayMontageAndWaitProxy` "None" "/Game/PlayerCharacter/Wraith/Animations/RunningSlide/short_sliding_anim_Montage.short_sliding_anim_Montage"
      (:`then`
        (`AbilityTask_WaitGameplayEvent.WaitGameplayEvent` (struct :`TagName` "Event.Montage.Slide") null
          (:`EventReceived`
            (`/Game/PlayerCharacter/Character/BP_PlayerCharacter.DisableSliding` _owner)
            (`AbilitySystemBlueprintLibrary.RemoveLooseGameplayTags` _owner (`BlueprintGameplayTagLibrary.MakeLiteralGameplayTagContainer` (struct :`GameplayTags` (struct :`(TagName` "State.Sliding")))))
            (`self.K2_EndAbility`))))
      (:`OnCompleted`
        (`self.K2_EndAbility` :!label _label))
      (:`OnBlendOut`
        (goto _label))
      (:`OnInterrupted`
        (goto _label))
      (:`OnCancelled`
        (goto _label)))))

(event `self.K2_OnEndAbility`
  (params (bWasCancelled :type Boolean))
  (bind _owner (`self.Owner`))
  (`SkinnedMeshComponent.UnHideBoneByName` (`Character.Mesh` (`self.Owner`)) "weapon_r")
  (`/Game/PlayerCharacter/Character/BP_PlayerCharacter.DisableSliding` _owner)
  (`AbilitySystemBlueprintLibrary.RemoveLooseGameplayTags` _owner (`BlueprintGameplayTagLibrary.MakeLiteralGameplayTagContainer` (struct :`GameplayTags` (struct :`(TagName` "State.Sliding")))))
  (`PrimitiveComponent.SetCollisionResponseToChannel` (`Character.CapsuleComponent` (`self.Owner`)) "ECC_GameTraceChannel1" "ECR_Block"))
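; BP_Bomb is a projectile bomb in the GAS bomb ability, instigated by a Wraith character.
; On overlap it stops moving, waits a configurable delay, then spawns FS_Bomb at its position.
; A debug-drawn, single-hit sphere trace then finds a player character, calls RunOnOwningClient with the Wraith, and applies GE_BombDamage through that player's Ability System Component.
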(event `self.ReceiveBeginPlay`
  (bind _asbp_wraith_character (cast `/Game/PlayerCharacter/Wraith/BP_WraithCharacter` (`self.Instigator`)))
  (set `self.Wraith` _asbp_wraith_character))

(event `self.CollsionDetection.OnComponentBeginOverlap`
  (params (OverlappedComponent :type "PrimitiveComponent Object Reference") (OtherActor :type "Actor Object Reference") (OtherComp :type "PrimitiveComponent Object Reference") (OtherBodyIndex :type Integer) (bFromSweep :type Boolean) (SweepResult :type "HitResult Structure (by ref)"))
  (bind _returnvalue (`SceneComponent.K2_GetComponentLocation` (`self.Sphere`)))
  (`ProjectileMovementComponent.StopSimulating` (`self.ProjectileMovement`) SweepResult)
  (`KismetSystemLibrary.Delay` (`self.DelayUntilExplosion`))
  (`|SpawnActorFromClass` "/Game/Chaos/Fields/FS_Bomb.FS_Bomb_C" (`KismetMathLibrary.MakeTransform` _returnvalue) "AlwaysSpawn" "MultiplyWithRoot" null null)
  (bind (_outhit _returnvalue_2) (`KismetSystemLibrary.SphereTraceSingle` :`Start` _returnvalue :`End` _returnvalue :`Radius` 1000.0 :`TraceChannel` "TraceTypeQuery1" :`DrawDebugType` "ForDuration"))
  (if _returnvalue_2
    (bind _asbp_player_character (cast `/Game/PlayerCharacter/Character/BP_PlayerCharacter` (`.HitActor` (`GameplayStatics.BreakHitResult` _outhit))))
    (`/Game/PlayerCharacter/Character/BP_PlayerCharacter.RunOnOwningClient` _asbp_player_character (`self.Wraith`))
    (bind _abilitysystemcomponent (`CLMCharacter.AbilitySystemComponent` _asbp_player_character))
    (`AbilitySystemComponent.BP_ApplyGameplayEffectSpecToSelf` _abilitysystemcomponent (`AbilitySystemComponent.MakeOutgoingSpec` :`self` _abilitysystemcomponent :`GameplayEffectClass` "/Game/GAS/BombAbility/GE_BombDamage.GE_BombDamage_C"))))

(fn `UserConstructionScript`)
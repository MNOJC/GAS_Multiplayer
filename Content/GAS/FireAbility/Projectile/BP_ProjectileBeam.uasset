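; Beam projectile for the GAS fire ability that faces EndLocation on spawn and flies straight toward it.
; Tick moves it with constant interpolation, raising speed every frame by a fixed, frame-rate-dependent step up to MaxSpeed.
; On a hit it plays an impact sound at arrival and destroys itself; on a miss it hides the beam short of the end and dissolves before destruction.
; EndLocation has an OnRep handler, currently empty.
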(event `self.ReceiveBeginPlay`
  (bind _returnvalue (`self.K2_GetActorLocation`))
  (`self.K2_SetActorLocationAndRotation` _returnvalue (`KismetMathLibrary.FindLookAtRotation` _returnvalue (`self.EndLocation`))))

(event `self.ReceiveTick`
  (params (DeltaSeconds :type "Float (single-precision)"))
  (bind _returnvalue (`self.K2_GetActorLocation`))
  (bind _endlocation (`self.EndLocation`))
  (bind _returnvalue_2 (`KismetMathLibrary.Vector_Distance` _returnvalue _endlocation))
  (`self.K2_SetActorLocationAndRotation` (`KismetMathLibrary.VInterpTo_Constant` _returnvalue _endlocation (`GameplayStatics.GetWorldDeltaSeconds`) (`self.CurrentSpeed`)) (`self.K2_GetActorRotation`))
  (set `self.CurrentSpeed` (`KismetMathLibrary.FClamp` (+ (`self.CurrentSpeed`) 50000.0) 0.0 (`self.MaxSpeed`)))
  (if (`self.Hit`)
    (if (< _returnvalue_2 1.0)
      (`/Engine/EditorBlueprintResources/StandardMacros.DoOnce` false
        (:`Completed`
          (`GameplayStatics.SpawnSoundAtLocation` "/Game/SFX/Weapon/Impact.Impact" (`self.EndLocation`) (struct) 0.3 1.0 0.0 "/Game/SFX/Attenuation/SA_Impact.SA_Impact" null)
          (`self.K2_DestroyActor`))))
    (elif (< _returnvalue_2 1000.0)
      (`/Engine/EditorBlueprintResources/StandardMacros.DoOnce` false
        (:`Completed`
          (`KismetSystemLibrary.PrintString` "Hello")
          (`SceneComponent.SetVisibility` (`self.Beam`) false false)
          (`ActorComponent.Activate` (`self.HitDissolve`) true)
          (`KismetSystemLibrary.Delay` 0.2)
          (`self.K2_DestroyActor`))))))

(fn `OnRep_EndLocation`)

(fn `UserConstructionScript`)
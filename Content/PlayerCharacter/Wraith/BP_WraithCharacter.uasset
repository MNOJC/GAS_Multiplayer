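; Wraith player character with a replicated beam weapon, built on the Gameplay Ability System.
; Tick drives a HUD crosshair from the projected TargetPoint and sends aim offsets through server and multicast events to the AnimInstance.
; Firing sphere-traces from the crosshair into beam impact data, with nearest-bone headshots, hit direction and local hit sounds.
; Server-to-multicast events spawn projectiles and test Chaos fields; effects handle delayed health regeneration and zero-energy overheat steam.
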(event `self.ReceiveBeginPlay`
  (`parent.ReceiveBeginPlay`)
  (bind _returnvalue (`KismetSystemLibrary.K2_SetTimerDelegate` (delegate `UpdateTargetPointLocation`) 1.0 true))
  (set `self.TimerInitHandle` _returnvalue))

(event `self.ReceiveTick`
  (params (DeltaSeconds :type "Float (single-precision)"))
  (bind _playercontroller (`self.PlayerController`))
  (bind _hud (`self.HUD`))
  (bind _screenposition (`WidgetLayoutLibrary.ProjectWorldLocationToWidgetPosition` _playercontroller (`SceneComponent.K2_GetComponentLocation` (`self.Target_Point`))))
  (bind _returnvalue (`KismetMathLibrary.Distance2D` _screenposition (`self.GetScreenCenterPos`)))
  (`parent.ReceiveTick` DeltaSeconds)
  (`|ExecutionSequence`
    (:`then_0`
      (if (`self.InitCompleted`)
        (if (not (`BlueprintGameplayTagLibrary.HasAnyTags` (`GameplayTagAssetInterface.GetOwnedGameplayTags` (`self.AbilitySystemComponent`)) (`BlueprintGameplayTagLibrary.MakeLiteralGameplayTagContainer` (struct :`GameplayTags` (struct :`(TagName` "Event.Death") :`(TagName` "State.Running") :`(TagName` "State.Sliding") :`(TagName` "Wallrun.CharacterIsAttached"))))))
          (`/Engine/EditorBlueprintResources/StandardMacros.IsValid` _playercontroller
            (:`Is Valid`
              (bind (_pitchoffset _yawoffset) (`PublicCPPLibrary.GetDynamicAimOffset` (`self.PlayerController`) (`self.Target_Point`) (`GameplayStatics.GetWorldDeltaSeconds`)))
              (`/Engine/EditorBlueprintResources/StandardMacros.IsValid` _hud
                (:`Is Valid`
                  (if (not (< (`KismetMathLibrary.Distance2D` _screenposition (`self.GetScreenCenterPos`)) 5.0))
                    (`self.Server_UpdateAimingOffset` _pitchoffset _yawoffset))
                  (if (< _returnvalue 80.0)
                    (set `self.DynamicCrossairPos` _screenposition))
                  (`/Game/Widget/WBP_HUD.UpdateTargetLoc` (`/Game/Core/MainMap/HUD_MainInterface.W_HUD` _hud) (`self.DynamicCrossairPos`) (`KismetMathLibrary.SelectFloat` 10.0 2.0 (< _returnvalue 30.0))))))))))
    (:`then_1`)))

(event `UpdateTargetPointLocation`
  (set `self.ScreenCenterPos` (`self.GetScreenCenterPos`))
  (set `self.InitCompleted` true)
  (`KismetSystemLibrary.K2_ClearAndInvalidateTimerHandle` (`self.TimerInitHandle`)))

(event `Server_UpdateAimingOffset`
  (params (Pitch_Offset :type "Float (double-precision)") (Yaw_Offset :type "Float (double-precision)"))
  ;[0 0 0] Aim offset netwwork
  (`self.MC_UpdateAimingOffset` Pitch_Offset Yaw_Offset))

(event `MC_UpdateAimingOffset`
  (params (Pitch_Offset :type "Float (double-precision)") (Yaw_Offset :type "Float (double-precision)"))
  ;[0 0 0] Aim offset netwwork
  (`self.UpdateAimingOffset` Pitch_Offset Yaw_Offset))

(event `UpdateImpact`
  ;[0 0 0] Impact Beam
  (bind _output_get (`self.UpdateFireImpactPoint`))
  (bind _output_get_2 (set `self.BeamImpactData` _output_get))
  (`self.ServerUpdateData` _output_get_2)
  (bind (_hit _hitactor _position _normal) (break `/Game/PlayerCharacter/Structures/S_BeamImpact` _output_get_2))
  (bind (_returnvalue_roll _returnvalue_pitch _returnvalue_yaw) (`KismetMathLibrary.BreakRotator` (`KismetMathLibrary.Conv_VectorToRotator` _normal)))
  ;[0 1 0.0125] Chaos testing
  (`self.Server_Actor` "/Game/Chaos/Fields/FS_HitDamage.FS_HitDamage_C" (`KismetMathLibrary.MakeTransform` _position (`KismetMathLibrary.MakeRotator` _returnvalue_roll (+ _returnvalue_pitch -90.0) _returnvalue_yaw))))

(event `StartHealthRegenCountdown`
  (bind _abilitysystemcomponent (`self.AbilitySystemComponent`))
  ;[0 0 0] Healing
  (`self.RemoveGameplayEffect` _abilitysystemcomponent "/Game/GAS/HitAbility/GE_LifeRegeneration.GE_LifeRegeneration_C")
  (`KismetSystemLibrary.RetriggerableDelay` (`self.TimeBeforeHealing`))
  (`AbilitySystemComponent.BP_ApplyGameplayEffectToSelf` :`self` _abilitysystemcomponent :`GameplayEffectClass` "/Game/GAS/HitAbility/GE_LifeRegeneration.GE_LifeRegeneration_C"))

(event `ServerUpdateData`
  (params (BeamImpactData :type "/Game/PlayerCharacter/Structures/S_BeamImpact Structure"))
  ;[0 0 0] Impact Beam
  (set `self.BeamImpactData` BeamImpactData))

(event `SpawnProjectile`
  (params (SpawnTransform :type "Transform Structure") (EndLocation :type "Vector Structure") (Hit :type Boolean))
  ;[0 0 0] Spawn actor replicated
  (`self.Server_SpawnActor` SpawnTransform EndLocation Hit))

(event `Server_SpawnActor`
  (params (SpawnTransform :type "Transform Structure") (EndLocation :type "Vector Structure") (Hit :type Boolean))
  ;[0 0 0] Spawn actor replicated
  (`self.MC_SpawnActor` SpawnTransform EndLocation Hit))

(event `SpawnReplicatedProjectile`
  (params (SpawnTransform :type "Transform Structure") (EndLocation :type "Vector Structure") (Hit :type Boolean))
  ;[0 0 0] Impact Beam
  (`/Engine/EditorBlueprintResources/ActorMacros.Switch Has Authority`
    (:`Authority`
      (`self.MC_SpawnBeam` SpawnTransform EndLocation Hit))))

(event `MC_SpawnBeam`
  (params (SpawnTransform :type "Transform Structure") (EndLocation :type "Vector Structure") (Hit :type Boolean))
  ;[0 0 0] Impact Beam
  (`|SpawnActorFromClass` "/Game/GAS/FireAbility/Projectile/BP_ProjectileBeam.BP_ProjectileBeam_C" SpawnTransform "AlwaysSpawn" "MultiplyWithRoot" null EndLocation Hit null))

(event `MC_SpawnActor`
  (params (SpawnTransform :type "Transform Structure") (EndLocation :type "Vector Structure") (Hit :type Boolean))
  ;[0 0 0] Spawn actor replicated
  (`|SpawnActorFromClass` "/Game/GAS/FireAbility/Projectile/BP_ProjectileBeam.BP_ProjectileBeam_C" SpawnTransform "Undefined" "MultiplyWithRoot" null EndLocation Hit null))

(event `Server_Actor`
  (params (Class :type "Actor Class Reference") (SpawnTransform :type "Transform Structure"))
  (`self.MC_Actor` Class SpawnTransform))

(event `MC_Actor`
  (params (Class :type "Actor Class Reference") (SpawnTransform :type "Transform Structure"))
  (`|SpawnActorFromClass` Class SpawnTransform "AdjustIfPossibleButAlwaysSpawn" "MultiplyWithRoot" null null))

(fn `Get Hit Direction`
  (params (Normal :type "Vector Structure") (HitActor :type "Actor Object Reference"))
  (returns (HitDirection :type "/Game/Enumeration/E_HitDirection Enum"))
  (locals (ForwardDot :type "Float (double-precision)" :default 0.0) (RightDot :type "Float (double-precision)"))
  (bind _forwarddot (`local.ForwardDot`))
  (bind _rightdot (`local.RightDot`))
  (set `local.ForwardDot` (`KismetMathLibrary.Dot_VectorVector` (`self.GetActorForwardVector` HitActor) Normal))
  (set `local.RightDot` (`KismetMathLibrary.Dot_VectorVector` (`self.GetActorRightVector` HitActor) Normal))
  (if (> _forwarddot 0.7)
    (return "NewEnumerator2")
    (elif (< _forwarddot -0.7)
      (return "NewEnumerator3")
      (elif (> _rightdot 0.7)
        (return "NewEnumerator1")
        (elif (< _rightdot -0.7)
          (return "NewEnumerator0")
          (else
            (return "NewEnumerator2")))))))

(fn `GetClosestBone`
  (params (Location :type "Vector Structure") (Actor :type "Actor Object Reference"))
  (returns (`Closest bone` :type Name) (isHeadShot :type Boolean))
  (locals (minDist :type "Float (double-precision)" :default 1e+24) (ClosestBone :type Name))
  (bind _closestbone (`local.ClosestBone`))
  (bind _ascharacter (cast `Character` Actor))
  (for _array_element (`self.Bone Names`)
    (bind _returnvalue (`KismetMathLibrary.Vector_Distance` Location (`SceneComponent.GetSocketLocation` (`Character.Mesh` _ascharacter) _array_element)))
    (if (< _returnvalue (`local.minDist`))
      (set `local.ClosestBone` _array_element)
      (set `local.minDist` _returnvalue)))
  (return _closestbone (== _closestbone "head")))

(fn `GetMaterialInstance`
  (returns (MaterialInstanced :type "Array of MaterialInstanceDynamic Object Reference"))
  (locals (MaterialInstance :type Integer))
  (bind _mesh (`self.Mesh`))
  (for _index (range 4)
    (bind _returnvalue (`PrimitiveComponent.CreateDynamicMaterialInstance` _mesh _index (`PrimitiveComponent.GetMaterial` _mesh _index) "None"))
    (`KismetArrayLibrary.Array_Add` (`self.MaterialInstanced`) _returnvalue))
  (return (`self.MaterialInstanced`)))

(fn `GetScreenCenterPos`
  (returns (ReturnValue :type "Vector2D Structure"))
  (bind (_viewportposition_x _viewportposition_y) (`KismetMathLibrary.BreakVector2D` (`SlateBlueprintLibrary.ScreenToViewport` (`WidgetLayoutLibrary.GetViewportSize`))))
  (return (`KismetMathLibrary.MakeVector2D` (/ _viewportposition_x 2.0) (/ _viewportposition_y 2.0))))

(fn `GetTargetLocation`
  (bind _target_point (`self.Target_Point`))
  (bind (_outhit _returnvalue) (`KismetSystemLibrary.LineTraceSingle` :`Start` (`SceneComponent.GetSocketLocation` (`self.Mesh`) "gun_barrel") :`End` (`SceneComponent.K2_GetComponentLocation` (`self.Target_Point`)) :`TraceChannel` "TraceTypeQuery1" :`DrawDebugType` "ForDuration"))
  (if _returnvalue
    (`SceneComponent.K2_SetRelativeLocation` _target_point (0.0 600.0 0.0) false false)
    (else
      (`SceneComponent.K2_SetRelativeLocation` _target_point (0.0 600.0 0.0) false false)))
  (return))

(fn `OnRep_BeamImpactData`)

(fn `OnRep_End Location`)

(fn `OnRep_Pitch Offset`
  (message `/Game/PlayerCharacter/Wraith/Interfaces/BPI_AnimBP.SetAimingOffset` (`SkeletalMeshComponent.GetAnimInstance` (`self.Mesh`)) (`self.Pitch Offset`) (`self.Yaw Offset`)))

(fn `OnRep_Yaw Offset`
  (message `/Game/PlayerCharacter/Wraith/Interfaces/BPI_AnimBP.SetAimingOffset` (`SkeletalMeshComponent.GetAnimInstance` (`self.Mesh`)) (`self.Pitch Offset`) (`self.Yaw Offset`)))

(fn `PlayCharacterHitSound(Local)`
  (params (Headshot :type Boolean) (Actor :type "Actor Object Reference"))
  (cast `Character` Actor
    (:`then`
      (if Headshot
        (`GameplayStatics.PlaySound2D` "/Game/SFX/Weapon/Headshot.Headshot" 1.0 1.0 0.0 null null)
        (else
          (`GameplayStatics.PlaySound2D` "/Game/SFX/Weapon/BodyHit.BodyHit" 1.0 1.0 0.0 null null)))
      (return))
    (:`CastFailed`
      (return))))

(fn `UpdateAimingOffset`
  (params (Pitch_Offset :type "Float (double-precision)") (Yaw_Offset :type "Float (double-precision)"))
  (set `self.Pitch Offset` (+ Pitch_Offset (`self.Pitch Offset`)))
  (set `self.Yaw Offset` (+ Yaw_Offset (`self.Yaw Offset`)))
  (message `/Game/PlayerCharacter/Wraith/Interfaces/BPI_AnimBP.SetAimingOffset` (`SkeletalMeshComponent.GetAnimInstance` (`self.Mesh`)) (`self.Pitch Offset`) (`self.Yaw Offset`)))

(fn `UpdateBeamImpact`
  (`self.UpdateFireImpactPoint`)
  (return))

(fn `UpdateEnergy`
  (params (NewEnergy :type "Float (single-precision)"))
  (`parent.UpdateEnergy` NewEnergy)
  (if (<= NewEnergy 0.0)
    (`self.WeaponOverheat`)))

(fn `UpdateFireImpactPoint`
  (returns (Output_Get :type "/Game/PlayerCharacter/Structures/S_BeamImpact Structure"))
  (bind _returnvalue (`WidgetLayoutLibrary.GetViewportScale`))
  (bind _beamimpactdata (`self.BeamImpactData`))
  (bind _playercontroller (`self.PlayerController`))
  (bind _hud (`self.HUD`))
  (bind _w_hud (`/Game/Core/MainMap/HUD_MainInterface.W_HUD` _hud))
  (bind (_x _y) (`KismetMathLibrary.BreakVector2D` (`/Game/Widget/WBP_HUD.GetTargetLoc` _w_hud)))
  (bind (_worldposition _worlddirection) (`GameplayStatics.DeprojectScreenToWorld` _playercontroller (`KismetMathLibrary.MakeVector2D` (* _returnvalue _x) (* _returnvalue _y))))
  (`/Engine/EditorBlueprintResources/StandardMacros.IsValid` _hud
    (:`Is Valid`
      (`/Engine/EditorBlueprintResources/StandardMacros.IsValid` _w_hud
        (:`Is Valid`
          (`/Engine/EditorBlueprintResources/StandardMacros.IsValid` _playercontroller
            (:`Is Valid`
              (bind (_outhit _returnvalue_2) (`KismetSystemLibrary.SphereTraceSingle` _worldposition (+ _worldposition (* _worlddirection 10000.0)) 5.0 "TraceTypeQuery1"))
              (if _returnvalue_2
                (bind (_bblockinghit _binitialoverlap _time _distance _location _impactpoint _normal _impactnormal _physmat _hitactor _hitcomponent _hitbonename _bonename _hititem _elementindex _faceindex _tracestart _traceend) (`GameplayStatics.BreakHitResult` _outhit))
                (bind (_closest_bone _isheadshot) (`self.GetClosestBone` _location _hitactor))
                (`self.PlayCharacterHitSound(Local)` _isheadshot _hitactor)
                (bind _hitdirection (`self.Get Hit Direction` _normal _hitactor))
                (bind _structout (setmembers `/Game/PlayerCharacter/Structures/S_BeamImpact` :`StructRef` _beamimpactdata :`Hit` true :`HitActor` _hitactor :`Position` _location :`Normal` _normal :`SurfaceType` (`PhysicalMaterial.SurfaceType` _physmat) :`isHeadshot` _isheadshot :`HitDirection` _hitdirection))
                (return _structout)
                (else
                  (bind _structout_2 (setmembers `/Game/PlayerCharacter/Structures/S_BeamImpact` :`StructRef` _beamimpactdata :`Hit` false :`HitActor` null :`Position` _traceend :`Normal` (0.0 0.0 0.0) :`SurfaceType` "SurfaceType_Default" :`isHeadshot` false))
                  (return _structout_2))))))))))

(fn `UserConstructionScript`
  (`parent.UserConstructionScript`))

(fn `WeaponOverheat`
  (`ActorComponent.Activate` (`self.P_Steam_A_Converted`) true))
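; Networked player character built on the Gameplay Ability System, with combat and run states, aiming, wall running, health and energy.
; Default abilities are granted on BeginPlay, and a spawned BP_Camera becomes the view target.
; State changes drive the anim instance, camera manager and shakes, while Server-to-multicast event pairs relay velocity, launches and montages.
; Tick runs wall detection and, while attached, sets curve-driven wall-run velocity; health feeds blood HUD and death ragdoll.
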(event `RemoveGameplayEffect`
  (params (InstigatorAbilitySystemComponent :type "AbilitySystemComponent Object Reference") (GameplayEffect :type "GameplayEffect Class Reference"))
  ;[0 0 0] Remove Specific Gameplay Effect
  (`AbilitySystemComponent.RemoveActiveGameplayEffectBySourceEffect` (`self.AbilitySystemComponent`) GameplayEffect InstigatorAbilitySystemComponent -1))

(event `self.OnLanded`
  (params (Hit :type "HitResult Structure (by ref)"))
  ;[0 0 0] Landed
  (`AbilitySystemComponent.TryActivateAbilityByClass` (`self.AbilitySystemComponent`) "/Game/GAS/JumpAbility/GA_StopJump.GA_StopJump_C" true)
  (`self.ResetAttach`))

(event `self.ReceiveTick`
  (params (DeltaSeconds :type "Float (single-precision)"))
  (`self.WallRun`))

(event `self.ReceiveBeginPlay`
  ;[0 0 0] Give default abilities
  (for _array_element (`self.DefaultAbilities`)
    (`AbilitySystemComponent.K2_GiveAbility` (`self.AbilitySystemComponent`) _array_element 0 -1))
  ;[0 0 0] HUD ref
  (bind _aspc_main_map (cast `/Game/Core/MainMap/PC_MainMap` (`self.GetController`)))
  (set `self.PlayerController` _aspc_main_map)
  (bind _ashud_main_interface (cast `/Game/Core/MainMap/HUD_MainInterface` (`PlayerController.GetHUD` _aspc_main_map)))
  (set `self.HUD` _ashud_main_interface)
  (bind _aspcm_player (cast `/Game/Camera/PCM_Player` (`PlayerController.PlayerCameraManager` (`self.PlayerController`))))
  (set `self.As PCM Player` _aspcm_player)
  (`self.InitMainCamera`))

(event `AIM`
  (bind _as_pcm_player (`self.As PCM Player`))
  ;[0 0 0] FOV
  ;;[0 0 0] Aim
  (`/Engine/EditorBlueprintResources/StandardMacros.IsValid` _as_pcm_player
    (:`Is Valid`
      (`/Game/Camera/PCM_Player.StartAiming` _as_pcm_player)
      (`self.AimingSensibility` true)
      (`self.AimingAudio`))))

(event `RunCamera`
  (bind _as_pcm_player (`self.As PCM Player`))
  ;[0 0 0] FOV
  (`/Engine/EditorBlueprintResources/StandardMacros.IsValid` _as_pcm_player
    (:`Is Valid`
      (`/Game/Camera/PCM_Player.StartSprinting` _as_pcm_player))))

(event `UnAIM`
  (bind _as_pcm_player (`self.As PCM Player`))
  ;[0 0 0] FOV
  ;;[0 0 0] Aim
  (`/Engine/EditorBlueprintResources/StandardMacros.IsValid` _as_pcm_player
    (:`Is Valid`
      (`/Game/Camera/PCM_Player.StopAiming` _as_pcm_player)
      (`self.AimingSensibility` false)
      (`self.UnAimingAudio`))))

(event `CombatCamera`
  (bind _as_pcm_player (`self.As PCM Player`))
  ;[0 0 0] FOV
  (`/Engine/EditorBlueprintResources/StandardMacros.IsValid` _as_pcm_player
    (:`Is Valid`
      (`/Game/Camera/PCM_Player.StopSprinting` _as_pcm_player))))

(event `Server_UpdateVelocity`
  (params (Velocity :type "Vector Structure"))
  ;[0 0 0] Velocity Update Network
  (`self.MC_UpdateVelocity` Velocity))

(event `UpdateLocomotionMode`
  (params (`Player State` :type "/Game/Enumeration/E_PlayerState Enum" :default "NewEnumerator0"))
  ;[0 0 0] Locomotion mode
  (`self.ChangeLocomotionMode` `Player State`)
  (`self.RPC_Server_ChangeLocomotionMode` (`self.Player State`)))

(event `OwningClient`
  (params (NewHealth :type "Float (double-precision)"))
  ;[0 0 0] Update blood
  (`self.UpdateBloodSplatter` NewHealth))

(event `MC_UpdateVelocity`
  (params (Velocity :type "Vector Structure"))
  ;[0 0 0] Velocity Update Network
  (set `MovementComponent.Velocity` Velocity (`self.CharacterMovement`)))

(event `RPC_Server_ChangeLocomotionMode`
  (params (`Player State` :type "/Game/Enumeration/E_PlayerState Enum" :default "NewEnumerator0"))
  ;[0 0 0] Locomotion mode
  (`self.RPC_MC_ChangeLocomotionMode` `Player State`))

(event `PlaySoundOnce`
  (params (Sound :type "SoundBase Object Reference"))
  ;[0 0 0] Sound once
  (`/Engine/EditorBlueprintResources/StandardMacros.DoOnce` false :!label _label
    (:`Completed`
      (`GameplayStatics.PlaySound2D` Sound 1.0 1.0 0.0 null null))))

(event `ResetSound`
  ;[0 0 0] Sound once
  (goto _label :!via `Reset`))

(event `Server_LaunchCharacter`
  (params (LaunchVelocity :type "Vector Structure") (bXYOverride :type Boolean) (bZOverride :type Boolean))
  ;[0 0 0] Launch Character Network
  (`self.MC_LaunchCharacter` LaunchVelocity bXYOverride bZOverride))

(event `Server_PlayMontage`
  (params (MontageToPlay :type "AnimMontage Object Reference") (PlayRate :type "Float (single-precision)"))
  ;[0 0 0] Montage Network
  (`self.MC_PlayMontage` MontageToPlay PlayRate))

(event `RPC_MC_ChangeLocomotionMode`
  (params (`Player State` :type "/Game/Enumeration/E_PlayerState Enum" :default "NewEnumerator0"))
  ;[0 0 0] Locomotion mode
  (`self.ChangeLocomotionMode` `Player State`))

(event `MC_PlayMontage`
  (params (MontageToPlay :type "AnimMontage Object Reference") (PlayRate :type "Float (single-precision)"))
  ;[0 0 0] Montage Network
  (`|PlayMontage` (`self.Mesh`) MontageToPlay PlayRate))

(event `MC_LaunchCharacter`
  (params (LaunchVelocity :type "Vector Structure") (bXYOverride :type Boolean) (bZOverride :type Boolean))
  ;[0 0 0] Launch Character Network
  (`self.LaunchCharacter` LaunchVelocity bXYOverride bZOverride))

(event `WallRun`
  (bind _normal (`self.Normal`))
  (bind _abilitysystemcomponent (`self.AbilitySystemComponent`))
  (bind _returnvalue (* _normal -1.0))
  (bind (_returnvalue_x _returnvalue_y) (`KismetMathLibrary.BreakVector` (* _returnvalue 100.0)))
  (bind (_returnvalue_x_2 _returnvalue_y_2) (`KismetMathLibrary.BreakVector` (* (`KismetMathLibrary.Cross_VectorVector` (`KismetMathLibrary.Vector_Up`) (`KismetMathLibrary.SelectVector` _normal _returnvalue (> (`self.TraceDirection`) 1.0))) 1250.0)))
  ;[0 0 0] WallRun
  (`AbilitySystemComponent.TryActivateAbilityByClass` _abilitysystemcomponent "/Game/GAS/WallrunAbility/GA_WallDetection.GA_WallDetection_C" true)
  (if (`GameplayTagAssetInterface.HasMatchingGameplayTag` _abilitysystemcomponent (struct :`TagName` "Wallrun.CharacterIsAttached"))
    (bind _output_get (set `self.WallrunTimer` (+ (`GameplayStatics.GetWorldDeltaSeconds`) (`self.WallrunTimer`))))
    (`self.Server_UpdateVelocity` (`KismetMathLibrary.MakeVector` (+ _returnvalue_x _returnvalue_x_2) (+ _returnvalue_y _returnvalue_y_2) (* (`CurveFloat.GetFloatValue` (`self.WallrunCurve`) _output_get) 100.0)))
    (else
      (set `self.WallrunTimer` 0.0))))

(event `InitMainCamera`
  ;[0 0 0] Init player camera
  (bind _returnvalue (`|SpawnActorFromClass` "/Game/Camera/BP_Camera.BP_Camera_C" (`KismetMathLibrary.MakeTransform` (`self.K2_GetActorLocation`)) "AdjustIfPossibleButAlwaysSpawn" "MultiplyWithRoot" null null))
  (bind _output_get (set `self.MainCamera` _returnvalue))
  (`/Engine/EditorBlueprintResources/StandardMacros.IsValid` _output_get
    (:`Is Valid`
      (bind _output_get_2 (set `/Game/Camera/BP_Camera.Player` self (`self.MainCamera`)))
      (`/Engine/EditorBlueprintResources/StandardMacros.IsValid` _output_get_2
        (:`Is Valid`
          (`KismetSystemLibrary.DelayUntilNextTick`)
          (`PlayerController.SetViewTargetWithBlend` (`self.PlayerController`) (`self.MainCamera`) 0.0 "VTBlend_Linear" 0.0 false))))))

(event `Server_UpdateMirrorWallAnim`
  (params (Mirror :type Boolean))
  ;[0 0 0] Server update mirror anim
  (`self.UpdateMirorWallAnim` Mirror))

(event `Server_StopMontage`
  (params (AnimMontage :type "AnimMontage Object Reference"))
  ;[0 0 0] Stop Montage Network
  (`self.MC_StopMontage` AnimMontage))

(event `MC_StopMontage`
  (params (AnimMontage :type "AnimMontage Object Reference"))
  ;[0 0 0] Stop Montage Network
  (`self.StopAnimMontage` AnimMontage))

(event `AttachPlayerToWall`
  ;[0 0 0] WallRun
  (`/Engine/EditorBlueprintResources/StandardMacros.DoOnce` false :!label _label_2
    (:`Completed`
      (`AbilitySystemComponent.TryActivateAbilityByClass` (`self.AbilitySystemComponent`) "/Game/GAS/WallrunAbility/GA_AttachToWall.GA_AttachToWall_C" true))))

(event `ResetAttach`
  ;[0 0 0] WallRun
  (goto _label_2 :!via `Reset`))

(event `Server_SetActive`
  (params (Target :type "ActorComponent Object Reference") (bNewActive :type Boolean) (bReset :type Boolean))
  (`self.MC_SetActive` Target bNewActive bReset))

(event `RotateCharacter`
  (params (`New Rotation Z (Yaw)` :type "Float (single-precision)"))
  ;[0 0 0] WallRun
  (`self.K2_SetActorRotation` (`KismetMathLibrary.MakeRotator` 0.0 0.0 `New Rotation Z (Yaw)`)))

(event `MC_SetActive`
  (params (Target :type "ActorComponent Object Reference") (bNewActive :type Boolean) (bReset :type Boolean))
  (`ActorComponent.SetActive` Target bNewActive bReset))

(fn `AimingAudio`
  (bind _audio (`self.Audio`))
  (`AudioComponent.SetSound` _audio "/Game/SFX/Aim/AimingScope.AimingScope")
  (`AudioComponent.FadeIn` _audio 0.1 1.0 0.0 "Linear")
  (`GameplayStatics.PlaySound2D` "/Game/SFX/Aim/Scope.Scope" 1.0 1.0 0.0 null null))

(fn `AimingSensibility`
  (params (Aiming :type Boolean))
  (bind _playercontroller (`self.PlayerController`))
  (if Aiming
    (set `/Game/Core/MainMap/PC_MainMap.HorizontalSensibility` 0.2 _playercontroller)
    (set `/Game/Core/MainMap/PC_MainMap.VerticalSensibility` 0.2 _playercontroller)
    (else
      (set `/Game/Core/MainMap/PC_MainMap.HorizontalSensibility` 0.3 _playercontroller)
      (set `/Game/Core/MainMap/PC_MainMap.VerticalSensibility` 0.3 _playercontroller)))
  (return))

(fn `CameraShakeRunning`
  (params (State :type "/Game/Enumeration/E_PlayerState Enum" :default "NewEnumerator0"))
  (bind _as_pcm_player (`self.As PCM Player`))
  (switch `/Game/Enumeration/E_PlayerState` State
    (:`NewEnumerator0`
      (`/Engine/EditorBlueprintResources/StandardMacros.IsValid` _as_pcm_player
        (:`Is Valid`
          (`PlayerCameraManager.StopAllCameraShakes` _as_pcm_player true))))
    (:`NewEnumerator1`
      (`LegacyCameraShake.StartLegacyCameraShake` _as_pcm_player "/Game/Camera/CameraShake/CS_Run.CS_Run_C"))))

(fn `ChangeCameraViewMode`
  (params (PlayerState :type "/Game/Enumeration/E_PlayerState Enum" :default "NewEnumerator0"))
  (switch `/Game/Enumeration/E_PlayerState` PlayerState
    (:`NewEnumerator0`
      (`self.CombatCamera`))
    (:`NewEnumerator1`
      (`self.RunCamera`)))
  (return))

(fn `ChangeLocomotionMode`
  (params (`Player State` :type "/Game/Enumeration/E_PlayerState Enum" :default "NewEnumerator0"))
  (`self.CameraShakeRunning` `Player State`)
  (`self.ChangeCameraViewMode` `Player State`)
  (bind _output_get (set `self.Player State` `Player State`))
  (bind _asabp_wraith_character (cast `/Game/PlayerCharacter/Wraith/Animations/Blueprint/ABP_WraithCharacter` (`SkeletalMeshComponent.GetAnimInstance` (`self.Mesh`))))
  (`/Game/PlayerCharacter/Wraith/Animations/Blueprint/ABP_WraithCharacter.UpdatePlayerState` _asabp_wraith_character _output_get))

(fn `GetCameraManager`
  (returns (`Camera Manager` :type "/Game/Camera/PCM_Player Object Reference"))
  (bind _aspcm_player (cast `/Game/Camera/PCM_Player` (`PlayerController.PlayerCameraManager` (`self.PlayerController`))))
  (return _aspcm_player))

(fn `OnRep_MirrorWallAnim`
  (message `/Game/PlayerCharacter/Wraith/Interfaces/BPI_AnimBP.UpdateMirrorWallAnim` (`SkeletalMeshComponent.GetAnimInstance` (`self.Mesh`)) (`self.MirrorWallAnim`)))

(fn `OnRep_Player State`
  (bind _asabp_wraith_character (cast `/Game/PlayerCharacter/Wraith/Animations/Blueprint/ABP_WraithCharacter` (`SkeletalMeshComponent.GetAnimInstance` (`self.Mesh`))))
  (`/Game/PlayerCharacter/Wraith/Animations/Blueprint/ABP_WraithCharacter.UpdatePlayerState` _asabp_wraith_character (`self.Player State`)))

(fn `SwitchSpeedEffect`
  (params (State :type "/Game/Enumeration/E_PlayerState Enum" :default "NewEnumerator0"))
  (bind _niagara (`/Game/Camera/BP_Camera.Niagara` (`self.MainCamera`)))
  (switch `/Game/Enumeration/E_PlayerState` State
    (:`NewEnumerator0`
      (`ActorComponent.SetActive` _niagara false true))
    (:`NewEnumerator1`
      (`ActorComponent.SetActive` _niagara true true))))

(fn `UnAimingAudio`
  (`AudioComponent.FadeOut` (`self.Audio`) 0.2 0.0 "Linear")
  (`GameplayStatics.PlaySound2D` "/Game/SFX/Aim/Unscope.Unscope" 1.0 1.0 0.0 null null))

(fn `UpdateBloodSplatter`
  (params (NewHealth :type "Float (double-precision)"))
  (bind _hud (`self.HUD`))
  (bind _w_blood (`/Game/Widget/WBP_HUD.W_Blood` (`/Game/Core/MainMap/HUD_MainInterface.W_HUD` _hud)))
  (`/Engine/EditorBlueprintResources/StandardMacros.IsValid` _hud
    (:`Is Valid`
      (if (< NewHealth 50.0)
        (if (> NewHealth 40.0)
          (`/Game/Widget/Blood/W_Blood.ChangeBloodState` _w_blood "NewEnumerator0")
          (`/Game/Widget/Blood/W_Blood.StartBlood` _w_blood 1.0)
          (elif (> NewHealth 20.0)
            (`/Game/Widget/Blood/W_Blood.ChangeBloodState` _w_blood "NewEnumerator1")
            (`/Game/Widget/Blood/W_Blood.StartBlood` _w_blood 1.2)
            (elif (> NewHealth 0.0)
              (`/Game/Widget/Blood/W_Blood.ChangeBloodState` _w_blood "NewEnumerator2")
              (`/Game/Widget/Blood/W_Blood.StartBlood` _w_blood 1.6))))
        (else
          (`/Game/Widget/Blood/W_Blood.StopBlood` _w_blood)))
      (return))))

(fn `UpdateEnergy`
  (params (NewEnergy :type "Float (single-precision)"))
  (`KismetSystemLibrary.PrintString` (`KismetStringLibrary.Conv_DoubleToString` NewEnergy))
  (if (<= NewEnergy 0.0)
    (`self.PlaySoundOnce` "/Game/SFX/Weapon/PowerDown_Cue.PowerDown_Cue")
    (elif (>= NewEnergy 100.0)
      (`self.ResetSound`)
      (`AbilitySystemBlueprintLibrary.AddLooseGameplayTags` self (`BlueprintGameplayTagLibrary.MakeLiteralGameplayTagContainer` (struct :`GameplayTags` (struct :`(TagName` "Event.EnergyFull")))) true))))

(fn `UpdateHealth`
  (params (NewHealth :type "Float (single-precision)"))
  (`self.OwningClient` NewHealth)
  (`KismetSystemLibrary.PrintString` (`KismetStringLibrary.Conv_DoubleToString` NewHealth) true true (struct :`R` 1.0 :`G` 0.022868 :`A` 1.0) 0.5)
  (if (<= NewHealth 0.0)
    (bind _returnvalue (`AbilitySystemComponent.TryActivateAbilityByClass` (`self.AbilitySystemComponent`) "/Game/GAS/DeathAbility/GA_Death.GA_Death_C" true))
    (if _returnvalue
      (`SkeletalMeshComponent.SetAllBodiesBelowSimulatePhysics` (`self.Mesh`) "pelvis" true true))))

(fn `UpdateMirorWallAnim`
  (params (Mirror :type Boolean))
  (bind _output_get (set `self.MirrorWallAnim` Mirror))
  (message `/Game/PlayerCharacter/Wraith/Interfaces/BPI_AnimBP.UpdateMirrorWallAnim` (`SkeletalMeshComponent.GetAnimInstance` (`self.Mesh`)) _output_get))

(fn `UserConstructionScript`)
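; BP_KillZone is a box trigger that returns player characters to a respawn location when they enter it.
; On overlap, it acts only on a BP_PlayerCharacter with a valid HUD, fading the screen through the HUD's fade widget.
; After a short delay, it passes the respawn manager's location for that player to ServerSetLocation, then waits again before calling FadeOut.
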(event `self.Box.OnComponentBeginOverlap`
  (params (OverlappedComponent :type "PrimitiveComponent Object Reference") (OtherActor :type "Actor Object Reference") (OtherComp :type "PrimitiveComponent Object Reference") (OtherBodyIndex :type Integer) (bFromSweep :type Boolean) (SweepResult :type "HitResult Structure (by ref)"))
  (bind _asbp_player_character (cast `/Game/PlayerCharacter/Character/BP_PlayerCharacter` OtherActor))
  (`/Engine/EditorBlueprintResources/StandardMacros.IsValid` _asbp_player_character
    (:`Is Valid`
      (bind _hud (`/Game/PlayerCharacter/Character/BP_PlayerCharacter.HUD` _asbp_player_character))
      (`/Engine/EditorBlueprintResources/StandardMacros.IsValid` _hud
        (:`Is Valid`
          (bind _wbp_fade (`/Game/Widget/WBP_HUD.WBP_Fade` (`/Game/Core/MainMap/HUD_MainInterface.W_HUD` _hud)))
          (`/Game/Widget/Fade/WBP_Fade.FadeIn` _wbp_fade)
          (`KismetSystemLibrary.Delay` 0.25)
          (`/Game/PlayerCharacter/Character/BP_PlayerCharacter.Server_SetLocation` _asbp_player_character _asbp_player_character (`/Game/PlayerCharacter/Blueprint/BP_RespawnManager.GetRespawnLocation` (`/Game/PlayerCharacter/Character/BP_PlayerCharacter.GetRespawnManager` _asbp_player_character) _asbp_player_character) false false)
          (`KismetSystemLibrary.Delay` 0.75)
          (`/Game/Widget/Fade/WBP_Fade.FadeOut` _wbp_fade))))))

(fn `UserConstructionScript`)
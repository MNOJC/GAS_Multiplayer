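; Custom character movement component that adds predicted sprint, slide and wall-run movement to the player character.
; It registers state flags and velocities as predicted properties on BeginPlay, with setter functions to update them.
; The max speed override raises speed while sprinting.
; CalcVelocity runs the parent calculation, then forces slide velocity or horizontal-only wall-run velocity, with a leftover debug print during wall runs.
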(event `self.ReceiveBeginPlay`
  ;[1 1 1] Register Predicted Properties on Begin Play
  (`self.AddPredictedProperty_Bool` "SprintVar")
  (`self.AddPredictedProperty_Vector` "SlideVelocity")
  (`self.AddPredictedProperty_Bool` "Slide")
  (`self.AddPredictedProperty_Vector` "WallRunVelocity")
  (`self.AddPredictedProperty_Bool` "WallRun"))

(event `self.K2_CalcVelocity`
  (params (deltaTime :type "Float (single-precision)") (Friction :type "Float (single-precision)") (bFluid :type Boolean) (BrakingDeceleration :type "Float (single-precision)"))
  (bind (_wallrunvelocity_x _wallrunvelocity_y) (`KismetMathLibrary.BreakVector` (`self.WallRunVelocity`)))
  (`parent.K2_CalcVelocity` deltaTime Friction bFluid BrakingDeceleration)
  (`|ExecutionSequence`
    (:`then_0`
      (if (`self.Slide`)
        (set `self.Velocity` (`self.SlideVelocity`))))
    (:`then_1`
      (if (`self.WallRun`)
        (set `self.Velocity` (`KismetMathLibrary.MakeVector` _wallrunvelocity_x _wallrunvelocity_y))
        (`KismetSystemLibrary.PrintString` "Hello")))))

(fn `K2_GetMaxSpeed`
  (returns (ReturnValue :type "Float (single-precision)"))
  (bind _returnvalue (`parent.K2_GetMaxSpeed`))
  (return (select `bool` (`self.SprintVar`) :`false` _returnvalue :`true` 900.0)))

(fn `SetSlide`
  (params (Velocity :type "Vector Structure") (Slide :type Boolean))
  (set `self.Slide` Slide)
  (set `self.SlideVelocity` Velocity))

(fn `SetSprint`
  (params (bSprint :type Boolean))
  (set `self.SprintVar` bSprint))

(fn `SetWallRun`
  (params (WallRun :type Boolean) (WallRunVelocity :type "Vector Structure"))
  (set `self.WallRun` WallRun)
  (set `self.WallRunVelocity` WallRunVelocity))
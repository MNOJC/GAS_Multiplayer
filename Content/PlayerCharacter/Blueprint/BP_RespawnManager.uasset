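; Respawn manager that picks where a player respawns, favoring the point farthest from the other players.
; GetRespawnLocation gathers all BP_WraithCharacter and BP_RespawnPoint actors, then sums each point's distance to every character except the respawning one.
; It returns the location of the point with the largest total and resets its working variables for the next call.
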(fn `GetRespawnLocation`
  (params (PlayerRespawned :type "CLMCharacter Object Reference"))
  (returns (Value :type "Vector Structure"))
  (locals (Players :type "Array of /Game/PlayerCharacter/Wraith/BP_WraithCharacter Object Reference") (CurrentDistance :type "Float (double-precision)" :default 0.0) (FarestDIstance :type "Float (double-precision)") (FarestPoint :type "/Game/PlayerCharacter/Blueprint/BP_RespawnPoint Object Reference") (Location :type "Vector Structure"))
  (bind _outactors (`GameplayStatics.GetAllActorsOfClass` "/Game/PlayerCharacter/Wraith/BP_WraithCharacter.BP_WraithCharacter_C"))
  (set `local.Players` _outactors)
  (bind _outactors_2 (`GameplayStatics.GetAllActorsOfClass` "/Game/PlayerCharacter/Blueprint/BP_RespawnPoint.BP_RespawnPoint_C"))
  (for _array_element _outactors_2
    (for _array_element_2 (`local.Players`)
      (if (not (== _array_element_2 PlayerRespawned))
        (set `local.CurrentDistance` (+ (`KismetMathLibrary.Vector_Distance` (`self.K2_GetActorLocation` _array_element) (`self.K2_GetActorLocation` _array_element_2)) (`local.CurrentDistance`)))))
    (if (> (`local.CurrentDistance`) (`local.FarestDIstance`))
      (set `local.FarestDIstance` (`local.CurrentDistance`))
      (set `local.FarestPoint` _array_element))
    (set `local.CurrentDistance` 0.0))
  (set `local.Location` (`self.K2_GetActorLocation` (`local.FarestPoint`)))
  (set `local.FarestDIstance` 0.0)
  (set `local.CurrentDistance` 0.0)
  (set `local.FarestPoint` null)
  (return (`local.Location`)))

(fn `UserConstructionScript`)
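; Weapon actor component that fires beam projectiles from the owning character toward the screen-center aim point.
; BeginPlay caches the owner as a Character and its PC_MainMap controller.
; Fire traces from the deprojected viewport center along the camera ray on the Visibility channel, returning the hit or trace end.
; It then spawns BP_ProjectileBeam at the mesh's Muzzle_01 socket, passing that end location and hit flag.
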(event `self.ReceiveBeginPlay`
  (bind _ascharacter (cast `Character` (`self.GetOwner`)))
  (set `self.As Character` _ascharacter)
  (bind _aspc_main_map (cast `/Game/Core/MainMap/PC_MainMap` (`Pawn.GetController` (`self.As Character`))))
  (set `self.Controller` _aspc_main_map))

(event `Fire`
  (bind (_returnvalue_location _returnvalue_rotation) (`KismetMathLibrary.BreakTransform` (`SceneComponent.GetSocketTransform` (`Character.Mesh` (`self.As Character`)) "Muzzle_01" "RTS_World")))
  (bind (_hitactor _bulletendposition _normal _surface_type _hit) (`self.GetFireImpactPoint`))
  (`|SpawnActorFromClass` "/Game/GAS/FireAbility/Projectile/BP_ProjectileBeam.BP_ProjectileBeam_C" (`KismetMathLibrary.MakeTransform` _returnvalue_location _returnvalue_rotation) "AdjustIfPossibleButAlwaysSpawn" "MultiplyWithRoot" null _bulletendposition _hit null))

(fn `GetFireImpactPoint`
  (returns (HitActor :type "Actor Object Reference") (BulletEndPosition :type "Vector Structure") (Normal :type "Vector Structure") (`Surface Type` :type "EPhysicalSurface Enum") (Hit :type Boolean))
  (bind (_returnvalue_x _returnvalue_y) (`KismetMathLibrary.BreakVector2D` (`WidgetLayoutLibrary.GetViewportSize`)))
  (bind (_worldposition _worlddirection) (`GameplayStatics.DeprojectScreenToWorld` (`self.Controller`) (`KismetMathLibrary.MakeVector2D` (* _returnvalue_x 0.5) (* _returnvalue_y 0.5))))
  (bind (_outhit _returnvalue) (`KismetSystemLibrary.LineTraceSingle` _worldposition (+ _worldposition (* _worlddirection 10000.0)) "TraceTypeQuery1"))
  (if _returnvalue
    (bind (_bblockinghit _binitialoverlap _time _distance _location _impactpoint _normal _impactnormal _physmat _hitactor _hitcomponent _hitbonename _bonename _hititem _elementindex _faceindex _tracestart _traceend) (`GameplayStatics.BreakHitResult` _outhit))
    (return _hitactor _location _normal (`PhysicalMaterial.SurfaceType` _physmat) true)
    (else
      (return null _traceend (0.0 0.0 0.0) "SurfaceType_Default" false))))